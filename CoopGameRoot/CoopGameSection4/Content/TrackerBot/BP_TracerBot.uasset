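; BP_TracerBot is a tracker bot Blueprint that visualizes a navigation path and scales its audio with movement speed.
; FindNextPathPoint synchronously finds a path from the bot to the first player controller actor and draws a debug sphere at each point, without moving the bot.
; Tick maps velocity magnitude to the Audio component's volume multiplier, so faster movement sounds louder.
; Nothing in this graph calls FindNextPathPoint or applies movement.
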(event Custom|FindNextPathPoint
  (bind _returnvalue (Class|NavigationSystemV1|FindPathtoActorSynchronously (Transformation|GetActorLocation) (Game|GetPlayerController 0) 5e+01 0 0))
  (for _array_element (Variables|/Script/NavigationSystem.NavigationPath|GetPathPoints _returnvalue)
    (Rendering|Debug|DrawDebugSphere _array_element 2e+01 12 "(R=0.000000,G=0.000000,B=1.000000,A=1.000000)" 1e+01 1.0)))

(event EventTick
  (params (DeltaSeconds :type Float%20%28single-precision%29))
  (Audio|Components|Audio|SetVolumeMultiplier (Variables|Default|GetAudio) (Math|Float|MapRangeClamped (Math|Vector|VectorLength (Transformation|GetVelocity)) 1e+01 1e+03 0.1 2.0) :!class /Script/Engine.AudioComponent))

(fn ConstructionScript)